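; Player controller for an outline demo that switches a Sobel outline post-process between stencil-based and depth-based variants.
; On BeginPlay it prints useful CVars and a mobile SceneColor format caveat, applies the stencil variant, and opens the control panel widget.
; The switch function creates a transient dynamic material instance, assigns it as the first PostProcessVolume's blendable, and prints the active mode.
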(event EventBeginPlay
  (Utilities|FlowControl|Sequence
    (:then_0
      (Development|PrintString "r.PostProcessing.DisableMaterials" true false "(R=0.000000,G=0.660000,B=1.000000,A=1.000000)" 5.0)
      (Development|PrintString "r.mobile.ForceDepthResolve" true false "(R=0.000000,G=0.660000,B=1.000000,A=1.000000)" 5.0)
      (Development|PrintString "r.CustomDepth" true false "(R=0.000000,G=0.660000,B=1.000000,A=1.000000)" 5.0)
      (Development|PrintString "r.mobile.SceneColorFormat" true false "(R=0.000000,G=0.660000,B=1.000000,A=1.000000)" 5.0)
      (Development|PrintString "Useful CVars:" true false "(R=0.000000,G=0.660000,B=1.000000,A=1.000000)" 5.0)
      (Development|PrintString "You might need to change shaders to sample from SceneDepth directly (instead of SceneColor.a) if using R11G11B10 as SceneColor's format, in mobile forward configuration." true false "(R=0.000000,G=0.660000,B=1.000000,A=1.000000)" 5.0))
    (:then_1
      (CallFunction|SetOutlinePostProcessMaterial true))
    (:then_2
      (bind _returnvalue (UserInterface|CreateWidget "/Game/Blueprints/WidgetBP_ControlPanel.WidgetBP_ControlPanel_C"))
      (bind _output_get (Variables|Default|SetControl%20Panel%20Widget%20BP _returnvalue))
      (UserInterface|Viewport|AddtoViewport _output_get 0))))

(fn ConstructionScript)

(fn SetOutlinePostProcessMaterial
  (params (UseStencilSobel :type Boolean))
  (Utilities|FlowControl|Sequence
    (:then_0
      (if UseStencilSobel
        (bind _returnvalue (Rendering|Material|CreateDynamicMaterialInstance (Variables|Default|GetOutlinePostProcessStencilMIC) "Stencil" "Transient" :!class /Script/Engine.KismetMaterialLibrary))
        (Variables|Default|SetOutlineMid _returnvalue)
        (else
          (bind _returnvalue_2 (Rendering|Material|CreateDynamicMaterialInstance (Variables|Default|GetOutlinePostProcessDepthMIC) "Depth" "Transient" :!class /Script/Engine.KismetMaterialLibrary))
          (Variables|Default|SetOutlineMid _returnvalue_2))))
    (:then_1
      (bind _outactors (Actor|GetAllActorsOfClass "/Script/Engine.PostProcessVolume"))
      (if (> (Utilities|Array|Length _outactors) 0)
        (Utilities|Struct|SetmembersinPostProcessSettings (Variables|/Script/Engine.PostProcessVolume|GetSettings (Utilities|Array|Get(acopy) _outactors)) (Utilities|Struct|MakeWeightedBlendables (Utilities|Array|MakeArray (Utilities|Struct|MakeWeightedBlendable 1.0 (Variables|Default|GetOutlineMid)))))
        (else
          (Development|PrintString "Post process volume not set correctly." true true "(R=1.000000,G=0.000000,B=0.000000,A=1.000000)"))))
    (:then_2
      (if UseStencilSobel
        (Development|PrintString "Switched to stencil sobel.")
        (else
          (Development|PrintString "Switched to depth sobel."))))))